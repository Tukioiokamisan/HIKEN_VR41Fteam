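; BP_GameReStartMenu is a VR restart menu actor whose Start and Quit options are triggered by grabbing their grab components.
; Grabbing Start shows a loading screen offset by the headset's height, waits briefly, then reloads or opens VRTemplateMap by name.
; Grabbing Quit exits the game.
; An unconnected chain that would notify BPC_GameManager, spawn a particle effect and destroy the actor never runs.
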(event `self.GrabComponentStart.OnGrabbed`
  (`XRLoadingScreenFunctionLibrary.SetLoadingScreen` "/Engine/EditorResources/AI/S_NavLink.S_NavLink" (4.0 4.0) (`KismetMathLibrary.MakeVector` 10.0 0.0 (/ (.z (`.DevicePosition` (`HeadMountedDisplayFunctionLibrary.GetOrientationAndPosition`))) 100.0)) false true) ; Offset values are in Meters
  (`KismetSystemLibrary.Delay` 3.0)
  (`GameplayStatics.OpenLevel` "VRTemplateMap"))

(event `self.GrabComponentQuit.OnGrabbed`
  (`KismetSystemLibrary.QuitGame` null "Quit"))

(fn `UserConstructionScript`)