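; Game manager component that runs the round timer, score and win or loss state.
; It counts tagged buildings and tracks their destruction ratio through OnDestroyed bindings, triggering game over once the target ratio is reached.
; Tick reads the timer and checks the externally set clear flag, pausing the timer when the round ends.
; Game clear adds an elapsed-time score and saves a top-three scoreboard to a BP_SaveScore slot.
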(event `self.ReceiveBeginPlay`
  ; BeginPlay処理（開始処理）
  (set `self.IsGameClear` false) ; ゲームクリアフラグを初期化
  (`self.EV_BuildingCount`) ; 破壊可能オブジェクトを検出
  (bind _outactors (`GameplayStatics.GetAllActorsWithTag` (`self.BuildTag`)))
  (for _array_element _outactors
    (add `Actor.OnDestroyed` _array_element (`|CreateDelegate` :!event `EV_BuildingDestroy`))))

(event `self.ReceiveTick`
  (params (DeltaSeconds :type "Float (single-precision)"))
  (bind _timer (`self.Timer`))
  ; Tick処理
  ;;[0.03112 0.07333 0.15 0.5] 制限時間処理
  (set `self.Time` (`KismetSystemLibrary.K2_GetTimerElapsedTimeHandle` _timer))
  (set `self.TimeLimit` (`KismetSystemLibrary.K2_GetTimerRemainingTimeHandle` _timer))
  ;;[0.000587 0.15 0.01008 0.5] ゲームクリア時処理を呼び出す
  (if (`self.IsGameClear`)
    (`KismetSystemLibrary.K2_PauseTimerHandle` (`self.Timer`))
    (`self.EV_GameClear`)
    (else
      ;;[0.15 0 0.001921 0.5] 現在のオブジェクト破壊率が目標を超えた場合、ゲームオーバー処理を呼び出す
      (if (>= (`self.DestroyProgress`) (`self.TargetProgress`))
        (`KismetSystemLibrary.K2_PauseTimerHandle` (`self.Timer`))
        (`self.EV_GameOver`)))))

(event `EV_Pause`
  (bind _timer (`self.Timer`))
  ; ゲームの制限時間のポーズ処理
  (if (`KismetSystemLibrary.K2_IsTimerPausedHandle` (`self.Timer`))
    (`KismetSystemLibrary.K2_UnPauseTimerHandle` _timer)
    (else
      (`KismetSystemLibrary.K2_PauseTimerHandle` _timer))))

(event `EV_GameStaet`
  ; ゲーム開始処理
  (bind _returnvalue (`KismetSystemLibrary.K2_SetTimerDelegate` (`|CreateDelegate` :!event `EV_TimeOver`) (`self.InputTimer`)))
  (set `self.Timer` _returnvalue)
  (set `self.IsGameClear` false)
  (`self.EV_BuildingCount`))

(event `EV_GameClear`
  ; ゲームクリア時処理
  ;;[0.0329 0.0103 0.15 0.5] 制限時間のスコア加算処理
  (`self.EV_AddScore` (* (`self.Time`) 100000.0))
  ;;[0.03467 0.15 0.03144 0.5] スコアの保存処理
  (`self.LoadGame` ; ロード処理
    (:`Output`
      (`self.UpdateScore` (`self.Score`) (`/Game/TeamContents/Yamaguchi/BP/BP_SaveScore.ScoreBoard` (`self.SaveData`))
        (:`Output`
          (`self.SaveGame`) ; セーブ処理
        )))))

(event `EV_TimeOver`
  ; ゲーム開始処理
  ;;[0.2698 0.01384 0.000226 0.5] 制限時間終了時処理
  (`self.EV_GameOver`))

(event `EV_GameOver`
  ; ゲームオーバー処理
)

(event `EV_AddScore`
  (params (Add_ScorePoint :type "Float (double-precision)"))
  ; スコア加算処理
  (set `self.Score` (+ Add_ScorePoint (`self.Score`))))

(event `EV_UpdateTimer`
  (params (`New Input Timer` :type "Float (double-precision)"))
  ; 制限時間を更新
  (set `self.InputTimer` `New Input Timer`))

(event `EV_BuildingCount`
  ; 破壊可能オブジェクトの総数をカウント
  (bind _outactors (`GameplayStatics.GetAllActorsWithTag` (`self.BuildTag`)))
  (bind _output_get (set `self.TotalBuildingCount` (`KismetArrayLibrary.Array_Length` _outactors)))
  (set `self.CurrntBuilding` _output_get)
  (set `self.DestroyProgress` 0.0))

(event `EV_OnBuildingDestroy`
  ; 破壊時のカウント・割合計算処理
  ;;[0 0.0114 0.15 0.5] 現在の破壊数をカウント
  (bind _result (`/Engine/EditorBlueprintResources/StandardMacros.DecrementInt` (`self.CurrntBuilding`) :!label _label)
    (:`  `
      (bind _output_get (set `self.CurrntBuilding` _result))
      ;;[0.00922 0.15 0 0.5] 現在の破壊率を計算
      (set `self.DestroyProgress` (- 1.0 (/ (`KismetMathLibrary.Conv_IntToDouble` _output_get) (`KismetMathLibrary.Conv_IntToDouble` (`self.TotalBuildingCount`))))))))

(event `EV_BuildingDestroy`
  (params (DestroyedActor :type "Actor Object Reference"))
  ; 破壊時のカウント・割合計算処理
  (goto _label))